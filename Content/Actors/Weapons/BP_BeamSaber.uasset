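; BP_BeamSaber is a melee beam saber weapon with a limited energy supply and a timed attack hitbox.
; While active, Tick drains energy by a per-second rate and deactivates the saber when it runs out.
; WeaponAttack briefly enables query-only collision, then disables it and clears the attack flag.
; Overlap logic sends damage to BP_CharacterBase actors, but its branch is fixed to false, so it never runs.
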(event `self.ReceiveBeginPlay`
  (`parent.ReceiveBeginPlay`))

(event `self.ReceiveTick`
  (params (DeltaSeconds :type "Float (single-precision)"))
  (if (`self.Activate`)
    (bind _output_get (set `self.LeftEnergy` (- (`self.LeftEnergy`) (* DeltaSeconds (`self.UseEnergyPerSec`)))))
    (if (<= _output_get 0.0)
      (set `self.Activate` false))))

(event `/Game/Actors/Weapons/BI_WeaponAction.WeaponAttack`
  (`PrimitiveComponent.SetCollisionEnabled` (`self.BeamSaberCollision`) "QueryOnly")
  (`KismetSystemLibrary.Delay` 0.7)
  (`PrimitiveComponent.SetCollisionEnabled` (`self.BeamSaberCollision`) "NoCollision")
  (set `self.bIsOnAttack` false))

(event `self.ReceiveActorBeginOverlap`
  (params (OtherActor :type "Actor Object Reference"))
  (if false
    (set `self.bIsOnAttack` true)
    (bind _asbp_character_base (cast `/Game/Actors/BP_CharacterBase` OtherActor))
    (bind _output_get (set `self.DamagedActor` _asbp_character_base))
    (message `/Game/Actors/BI_ActorGetAttack.GetDamage` _output_get (`self.BeamSaberDamage`))))

(fn `UserConstructionScript`)