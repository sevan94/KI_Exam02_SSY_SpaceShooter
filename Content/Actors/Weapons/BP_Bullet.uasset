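; BP_Bullet is a projectile actor that damages the first Character it overlaps.
; On BeginPlay it pushes its Sphere component forward with an impulse scaled by ShootSpeed and sets its lifespan to BulletExistTime.
; Overlapping a Character sends Damage through GetDamageMessage, spawns a scaled-down fireball explosion and destroys the bullet.
; Overlaps with other actor types are ignored.
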(event `self.ReceiveBeginPlay`
  (`PrimitiveComponent.AddImpulse` (`self.Sphere`) (* (`self.GetActorForwardVector`) (`self.ShootSpeed`)) "None" false)
  (`self.SetLifeSpan` (`self.BulletExistTime`)))

(event `self.ReceiveActorBeginOverlap`
  (params (OtherActor :type "Actor Object Reference"))
  (bind `_as캐릭터` (cast `Character` OtherActor))
  (bind _output_get (set `self.ActorToGetDamage` `_as캐릭터`))
  (message `/Game/Actors/BI_ActorGetAttack.GetDamage` _output_get (`self.Damage`))
  (`self.HitEffect`)
  (`self.K2_DestroyActor`))

(event `HitEffect`
  (`GameplayStatics.SpawnEmitterAtLocation` "/Game/ExampleContent/Blueprint_Communication/Effects/P_Explosion_Fireball.P_Explosion_Fireball" (`self.K2_GetActorLocation`) (struct) (0.3 0.3 0.3)))

(fn `UserConstructionScript`)