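; Weapon manager that handles a parent BP_CharacterBase's switching between beam rifle, normal rifle and beam saber, along with attack and reload input.
; On BeginPlay it caches the parent character and builds the weapon array.
; Swapping cycles the index, changes the class of the character's BPWeaponBase child actor and attaches the array's weapon at the WeaponSoket socket.
; Attack and Reload forward messages to the current array weapon.
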(event `self.ReceiveBeginPlay`
  (bind _asbp_character_base (cast `/Game/Actors/BP_CharacterBase` (`self.GetParentActor`)))
  (set `self.ParentCharacter` _asbp_character_base)
  (set `self.Weapons` (`|MakeArray` (`self.WeaponBeamRifle`) (`self.WeaponNormalRifle`) (`self.WeaponBeamSaber`) :!type "Actor Object Reference")))

(event `SwapWeapon`
  (bind _output (`|GetArrayItem` (`self.Weapons`) (`self.NowWeapon`)))
  ; 무기를 지정할 번호 1증가. 해당 번호로 배열에 접근.
  (set `self.NowWeapon` (mod (+ (`self.NowWeapon`) 1) (`self.WeaponsCount`)))
  (`ChildActorComponent.SetChildActorClass` (`/Game/Actors/BP_CharacterBase.BP_WeaponBase` (`self.ParentCharacter`)) (`GameplayStatics.GetObjectClass` _output))
  (`self.K2_AttachToActor` _output (`self.ParentCharacter`) "WeaponSoket" "KeepRelative" "KeepRelative" "KeepRelative" true))

(event `Attack`
  (message `/Game/Actors/Weapons/BI_WeaponAction.WeaponAttack` (`|GetArrayItem` (`self.Weapons`) (`self.NowWeapon`))))

(event `Reload`
  (message `/Game/Actors/Weapons/BI_WeaponAction.WeaponReload` (`|GetArrayItem` (`self.Weapons`) (`self.NowWeapon`))))

(event `EnhancedInput|/Game/Input/IA_WeaponSwap`
  (params (ActionValue :type Boolean) (ElapsedSeconds :type "Float (double-precision)") (TriggeredSeconds :type "Float (double-precision)") (InputAction :type "InputAction Object Reference" :default "/Game/Input/IA_WeaponSwap.IA_WeaponSwap"))
  (:`Triggered`
    (`self.SwapWeapon`)))

(event `EnhancedInput|/Game/Input/IA_Reload`
  (params (ActionValue :type Boolean) (ElapsedSeconds :type "Float (double-precision)") (TriggeredSeconds :type "Float (double-precision)") (InputAction :type "InputAction Object Reference" :default "/Game/Input/IA_Reload.IA_Reload"))
  (:`Triggered`
    (`self.Reload`)))

(event `EnhancedInput|/Game/Input/IA_Attack`
  (params (ActionValue :type Boolean) (ElapsedSeconds :type "Float (double-precision)") (TriggeredSeconds :type "Float (double-precision)") (InputAction :type "InputAction Object Reference" :default "/Game/Input/IA_Attack.IA_Attack"))
  (:`Triggered`
    (`self.Attack`)))

(fn `UserConstructionScript`)