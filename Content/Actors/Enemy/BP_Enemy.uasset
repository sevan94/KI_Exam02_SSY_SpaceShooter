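; BP_Enemy is an enemy actor that moves, takes damage and explodes on death.
; SeePlayer and Attackable use sphere overlaps at SightRadius and AttackRange to return a BP_Player, while MovetoPlayer adds movement input toward a given location.
; GetDamage lowers health and clears IsAlive at zero, after which Tick spawns an explosion emitter and destroys the actor.
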(event `/Game/Actors/Enemy/BI_AiAction.MoveToPlayer`
  (params (LocationToGo :type "Vector Structure"))
  (`self.AddMovementInput` (- LocationToGo (`self.K2_GetActorLocation`))))

(event `/Game/Actors/BI_ActorGetAttack.GetDamage`
  (params (Damage :type "Float (double-precision)"))
  (bind _output_get (set `self.Health_0` (- (`self.Health_0`) Damage)))
  (if (<= _output_get 0.0)
    (set `self.bIsAlive` false)))

(event `self.ReceiveTick`
  (params (DeltaSeconds :type "Float (single-precision)"))
  (if (not (`self.bIsAlive`))
    (`GameplayStatics.SpawnEmitterAtLocation` "/Game/Effect/Blueprint_Communication/Effects/P_Explosion_Bomb.P_Explosion_Bomb" (`self.K2_GetActorLocation`))
    (`self.K2_DestroyActor`)))

(fn `Attackable`
  (returns (OutActor :type "Actor Object Reference"))
  (bind (_outactors _returnvalue) (`KismetSystemLibrary.SphereOverlapActors` (`self.K2_GetActorLocation`) (`self.AttackRange`) (`|MakeArray` "ObjectTypeQuery3" :!type "EObjectTypeQuery Enum") "/Game/Actors/Player/BP_Player.BP_Player_C"))
  (if _returnvalue
    (return (`|GetArrayItem` _outactors))
    (else
      (return null))))

(fn `SeePlayer`
  (returns (OutTarget :type "Actor Object Reference"))
  (bind (_outactors _returnvalue) (`KismetSystemLibrary.SphereOverlapActors` (`self.K2_GetActorLocation`) (`self.SightRadius`) (`|MakeArray` "ObjectTypeQuery3" :!type "EObjectTypeQuery Enum") "/Game/Actors/Player/BP_Player.BP_Player_C"))
  (if _returnvalue
    (return (`|GetArrayItem` _outactors))
    (else
      (return null))))

(fn `UserConstructionScript`)