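; BP_BattleShip is an enemy battleship actor that takes damage and triggers a FinishGame event when destroyed.
; GetDamage subtracts from Hp and updates an IsAvailable flag, which Tick polls each frame.
; Once Hp is depleted, Tick spawns a bomb explosion emitter, calls the FinishGame dispatcher and destroys the actor.
; The ship binds its own FinishGame handler at BeginPlay, but that handler is empty.
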(event `self.ReceiveBeginPlay`
  (add `self.FinishGame` (delegate `FinishGame_Event`)))

(event `FinishGame_Event`)

(event `/Game/Actors/BI_ActorGetAttack.GetDamage`
  (params (Damage :type "Float (double-precision)"))
  (bind _output_get (set `self.Hp` (- (`self.Hp`) Damage)))
  (set `self.bIsAvailable` (> _output_get 0.0)))

(event `self.ReceiveTick`
  (params (DeltaSeconds :type "Float (single-precision)"))
  (if (not (`self.bIsAvailable`))
    (`GameplayStatics.SpawnEmitterAtLocation` "/Game/Effect/Blueprint_Communication/Effects/P_Explosion_Bomb.P_Explosion_Bomb" (`self.K2_GetActorLocation`))
    (`self.FinishGame`)
    (`self.K2_DestroyActor`)))

(fn `UserConstructionScript`)