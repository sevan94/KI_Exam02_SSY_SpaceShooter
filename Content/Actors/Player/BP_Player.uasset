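; BP_Player is the player character, flying freely in six directions with boost, zoom and weapon controls through Enhanced Input.
; Movement input follows actor axes horizontally and world Z vertically, while look input applies local pitch and yaw.
; Boost raises MaxFlySpeed and drains on Tick until released or empty, and zoom switches spring arm length.
; Attack, reload and swap go to a child-actor BP_WeaponManager, with a timed IsReloading flag.
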(event `EnhancedInput|/Game/Input/IA_RightLeft`
  (params (ActionValue :type "Float (double-precision)") (ElapsedSeconds :type "Float (double-precision)") (TriggeredSeconds :type "Float (double-precision)") (InputAction :type "InputAction Object Reference" :default "/Game/Input/IA_RightLeft.IA_RightLeft"))
  ; 좌우 움직임
  (:`Triggered`
    (`self.AddMovementInput` (* ActionValue (`self.GetActorRightVector`)))))

(event `EnhancedInput|/Game/Input/IA_FrontBack`
  (params (ActionValue :type "Float (double-precision)") (ElapsedSeconds :type "Float (double-precision)") (TriggeredSeconds :type "Float (double-precision)") (InputAction :type "InputAction Object Reference" :default "/Game/Input/IA_FrontBack.IA_FrontBack"))
  ; 정면으로 움직임
  (:`Triggered`
    (`self.AddMovementInput` (* ActionValue (`self.GetActorForwardVector`)))))

(event `EnhancedInput|/Game/Input/IA_Up`
  (params (ActionValue :type Boolean) (ElapsedSeconds :type "Float (double-precision)") (TriggeredSeconds :type "Float (double-precision)") (InputAction :type "InputAction Object Reference" :default "/Game/Input/IA_Up.IA_Up"))
  ; 위로 올라가는 동작
  (:`Triggered`
    (if ActionValue
      (bind _output_get (set `self.Direction` (`KismetMathLibrary.MakeVector` 0.0 0.0 (`self.TrueAsNumber`))))
      (`self.AddMovementInput` _output_get))))

(event `EnhancedInput|/Game/Input/IA_Down`
  (params (ActionValue :type Boolean) (ElapsedSeconds :type "Float (double-precision)") (TriggeredSeconds :type "Float (double-precision)") (InputAction :type "InputAction Object Reference" :default "/Game/Input/IA_Down.IA_Down"))
  ; 아래로 내려가는 동작
  (:`Triggered`
    (if ActionValue
      (bind _output_get (set `self.Direction` (`KismetMathLibrary.MakeVector` 0.0 0.0 (* (`self.TrueAsNumber`) (`self.Reverse`)))))
      (`self.AddMovementInput` _output_get))))

(event `BoostActive`
  ; 부스트 활성화
  (`self.IsBoostLeft`
    (:`True`
      (set `CharacterMovementComponent.MaxFlySpeed` (`self.BoostSpeed`) (`self.CharacterMovement`))
      (set `self.bIsBoosting` true))))

(event `BoostDeactive`
  ; 부스트 비활성화
  (set `CharacterMovementComponent.MaxFlySpeed` (`self.NormalSpeed`) (`self.CharacterMovement`))
  (set `self.bIsBoosting` false))

(event `self.ReceiveBeginPlay`
  ; 기본 움직임 속도 설정
  (set `CharacterMovementComponent.MaxFlySpeed` (`self.NormalSpeed`) (`self.CharacterMovement`))
  ; WeaponManager 초기화
  (bind _asbp_weapon_manager (cast `/Game/Actors/Weapons/BP_WeaponManager` (`ChildActorComponent.ChildActor` (`self.BP_WeaponManager`))))
  (set `self.WeaponManager` _asbp_weapon_manager))

(event `EnhancedInput|/Game/Input/IA_Boost`
  (params (ActionValue :type Boolean) (ElapsedSeconds :type "Float (double-precision)") (TriggeredSeconds :type "Float (double-precision)") (InputAction :type "InputAction Object Reference" :default "/Game/Input/IA_Boost.IA_Boost"))
  (:`Started`
    (`self.BoostActive`))
  (:`Completed`
    (`self.BoostDeactive`)))

(event `self.ReceiveTick`
  (params (DeltaSeconds :type "Float (single-precision)"))
  ; 부스트 활성화시 부스트 소모
  (if (`self.bIsBoosting`)
    (set `self.LeftBoostAmount` (- (`self.LeftBoostAmount`) (* DeltaSeconds (`self.UseBoostPerSecond`))))
    (`self.IsBoostLeft`
      (:`True`
        _)
      (:`False`
        (`self.BoostDeactive`)))
    (`KismetSystemLibrary.PrintString` (`KismetStringLibrary.Conv_DoubleToString` (`self.LeftBoostAmount`)))))

(event `EnhancedInput|/Game/Input/IA_TurnSight`
  (params (ActionValue :type "Vector Structure") (ElapsedSeconds :type "Float (double-precision)") (TriggeredSeconds :type "Float (double-precision)") (InputAction :type "InputAction Object Reference" :default "/Game/Input/IA_TurnSight.IA_TurnSight"))
  ; 회전
  (:`Triggered`
    (`self.K2_AddActorLocalRotation` (`KismetMathLibrary.MakeRotator` 0.0 ActionValue_Y ActionValue_X))))

(event `EnhancedInput|/Game/Input/IA_Zoom`
  (params (ActionValue :type Boolean) (ElapsedSeconds :type "Float (double-precision)") (TriggeredSeconds :type "Float (double-precision)") (InputAction :type "InputAction Object Reference" :default "/Game/Input/IA_Zoom.IA_Zoom"))
  ; 줌인
  (:`Started`
    (`self.ZoomActivate`))
  (:`Completed`
    (`self.ZoomDeactivate`)))

(event `ZoomActivate`
  ; 줌인
  (set `SpringArmComponent.TargetArmLength` (`self.ZoomSpringArm`) (`self.SpringArm`)))

(event `ZoomDeactivate`
  ; 줌인
  (set `SpringArmComponent.TargetArmLength` (`self.NormalSpringArm`) (`self.SpringArm`)))

(event `EnhancedInput|/Game/Input/IA_Attack`
  (params (ActionValue :type Boolean) (ElapsedSeconds :type "Float (double-precision)") (TriggeredSeconds :type "Float (double-precision)") (InputAction :type "InputAction Object Reference" :default "/Game/Input/IA_Attack.IA_Attack"))
  (:`Started`
    (`/Game/Actors/Weapons/BP_WeaponManager.Attack` (`self.WeaponManager`))))

(event `EnhancedInput|/Game/Input/IA_Reload`
  (params (ActionValue :type Boolean) (ElapsedSeconds :type "Float (double-precision)") (TriggeredSeconds :type "Float (double-precision)") (InputAction :type "InputAction Object Reference" :default "/Game/Input/IA_Reload.IA_Reload"))
  (:`Started`
    (set `self.bIsReloading` true)
    (`/Game/Actors/Weapons/BP_WeaponManager.Reload` (`self.WeaponManager`))
    (`KismetSystemLibrary.Delay` (`self.ReloadingTime`))
    (set `self.bIsReloading` false)))

(event `EnhancedInput|/Game/Input/IA_WeaponSwap`
  (params (ActionValue :type Boolean) (ElapsedSeconds :type "Float (double-precision)") (TriggeredSeconds :type "Float (double-precision)") (InputAction :type "InputAction Object Reference" :default "/Game/Input/IA_WeaponSwap.IA_WeaponSwap"))
  (:`Started`
    (`/Game/Actors/Weapons/BP_WeaponManager.SwapWeapon` (`self.WeaponManager`))))

(fn `UserConstructionScript`)